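; BP_RectangleSpawn is a breakable Geometry Collection rectangle that drops a random power-up.
; A hit from the first-person character, matched by display name, spawns a BP_UpDamage at the root, sets its activation type and calls CETrigger.
; The first Chaos break event, guarded by IsBroken, plays a collapse sound and runs GenerateItem to spawn one of four power-up cube variants at random.
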(event OnComponentHit(Rectangle_GeometryCollection)
  (params (HitComponent :type Primitive%20Component%20Object%20Reference) (OtherActor :type Actor%20Object%20Reference) (OtherComp :type Primitive%20Component%20Object%20Reference) (NormalImpulse :type Vector :default "0, 0, 0") (Hit :type Hit%20Result%20Structure%20%28by%20ref%29))
  (if (Utilities|Enum|Equal(Enum) (Utilities|GetDisplayName OtherActor) "BP_FirstPersonCharacter0")
    (bind _returnvalue (Game|SpawnActorfromClass "/Game/Blueprints/BP_UpDamage.BP_UpDamage_C" (Transformation|GetWorldTransform (Variables|Default|GetDefaultSceneRoot)) "Undefined" 0 0))
    (Variables|/Game/Blueprints/BP_UpDamage.BP_UpDamage_C|SetActivationType _returnvalue "NewEnumerator3")
    (Default|CETrigger _returnvalue)))

(event OnChaosBreakEvent(Rectangle_GeometryCollection)
  (params (BreakEvent :type Chaos%20Break%20Event%20Structure%20%28by%20ref%29))
  (if (not (Variables|Default|GetisBroken))
    (Variables|Default|SetisBroken true)
    (CallFunction|GenerateItem)
    (Audio|PlaySoundatLocation "/Game/StarterContent/Audio/Collapse01.Collapse01" "0, 0, 0" "0, 0, 0" 0.5 1.0 0.0 0 0 0 0)))

(event Custom|Generate%20Item
  (bind _defaultsceneroot (Variables|Default|GetDefaultSceneRoot))
  (bind _returnvalue (Transformation|GetRelativeTransform _defaultsceneroot))
  (switch int (Math|Random|RandomInteger 4)
    (:0
      (Game|SpawnActorfromClass "/Game/FirstPerson/Blueprints/BP_PowerUp_Cube.BP_PowerUp_Cube_C" _returnvalue "AlwaysSpawn" 0 0))
    (:1
      (Game|SpawnActorfromClass "/Game/FirstPerson/Blueprints/BP_PowerUp_Cube_2.BP_PowerUp_Cube_2_C" _returnvalue "AlwaysSpawn" 0 0))
    (:2
      (Game|SpawnActorfromClass "/Game/FirstPerson/Blueprints/BP_PowerUp_Cube_3.BP_PowerUp_Cube_3_C" _returnvalue "AlwaysSpawn" 0 0))
    (:3
      (Game|SpawnActorfromClass "/Game/FirstPerson/Blueprints/BP_PowerUp_Cube_4.BP_PowerUp_Cube_4_C" _returnvalue "AlwaysSpawn" 0 0))))

(event EventBeginPlay)

(event Collision|EventActorBeginOverlap
  (params (OtherActor :type Actor%20Object%20Reference)))

(event EventTick
  (params (DeltaSeconds :type Float%20%28single-precision%29)))

(fn ConstructionScript)