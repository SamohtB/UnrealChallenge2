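; Red cube destructible that counts hits on its Geometry Collection and explodes once accumulated damage passes a small threshold.
; A Sphere attached to the collection at BeginPlay sets the center and radius of the blast.
; Explode plays a collapse sound, then applies Chaos fields: external strain to break clusters, and a radial linear force culled outside the sphere to scatter pieces.
; Damage never resets, so every hit after the threshold triggers another explosion.
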(event OnComponentHit(RedCube_GeometryCollection)
  (params (HitComponent :type Primitive%20Component%20Object%20Reference) (OtherActor :type Actor%20Object%20Reference) (OtherComp :type Primitive%20Component%20Object%20Reference) (NormalImpulse :type Vector :default "0, 0, 0") (Hit :type Hit%20Result%20Structure%20%28by%20ref%29))
  (bind _damage (Variables|Default|GetDamage))
  (if (> _damage 4)
    (CallFunction|Explode)
    (else
      (Math|Integer|IncrementInt _damage))))

(event Custom|Explode
  (bind _fieldsystemcomponent (Variables|Field|GetFieldSystemComponent))
  (bind _radialfalloff (Variables|Default|GetRadialFalloff))
  (bind _sphere (Variables|Default|GetSphere))
  (bind _returnvalue (Components|Sphere|GetScaledSphereRadius _sphere))
  (bind _returnvalue_2 (Transformation|GetWorldLocation _sphere))
  (bind _returnvalue_3 (Field|SetRadialFalloff _radialfalloff 2e+09 0.0 1.0 0.0 _returnvalue _returnvalue_2 "Field_FallOff_None"))
  (Audio|PlaySoundatLocation "/Game/StarterContent/Audio/Collapse01.Collapse01" (Transformation|GetActorLocation) "0, 0, 0" 1.0 1.0 0.0 0 0 0 0)
  (Class|FieldSystemComponent|ApplyPhysicsField _fieldsystemcomponent true "Field_ExternalClusterStrain" 0 _returnvalue_3)
  (Class|FieldSystemComponent|ApplyPhysicsField _fieldsystemcomponent true "Field_LinearForce" 0 (Field|SetCullingField (Variables|Default|GetCullingField) _returnvalue_3 (Field|SetRadialVector (Variables|Default|GetRadialVector) 9e+07 _returnvalue_2) "Field_Culling_Outside")))

(event EventBeginPlay
  (Transformation|AttachComponentToComponent (Variables|Default|GetSphere) (Variables|Default|GetRedCube_GeometryCollection) "None" "KeepRelative" "KeepRelative" "KeepRelative" true))

(event Collision|EventActorBeginOverlap
  (params (OtherActor :type Actor%20Object%20Reference)))

(event EventTick
  (params (DeltaSeconds :type Float%20%28single-precision%29)))

(fn ConstructionScript)