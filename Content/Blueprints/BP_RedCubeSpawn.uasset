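; BP_RedCubeSpawn is a breakable red cube actor built on a Chaos Geometry Collection.
; On BeginPlay it spawns a BP_UpDamage actor at its root transform, sets that actor's activation type and immediately triggers it.
; The first Chaos break event, guarded by an IsBroken flag, plays a collapse sound and destroys the cube after a short delay.
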(event OnChaosBreakEvent(RedCube_GeometryCollection)
  (params (BreakEvent :type Chaos%20Break%20Event%20Structure%20%28by%20ref%29))
  (if (not (Variables|Default|GetisBroken))
    (Variables|Default|SetisBroken true)
    (Audio|PlaySoundatLocation "/Game/StarterContent/Audio/Collapse01.Collapse01" "0, 0, 0" "0, 0, 0" 0.5 1.0 0.0 0 0 0 0)
    (Utilities|FlowControl|Delay 5.0)
    (Actor|DestroyActor)))

(event EventBeginPlay
  (bind _returnvalue (Game|SpawnActorfromClass "/Game/Blueprints/BP_UpDamage.BP_UpDamage_C" (Transformation|GetWorldTransform (Variables|Default|GetDefaultSceneRoot)) "Undefined" 0 0))
  (Variables|/Game/Blueprints/BP_UpDamage.BP_UpDamage_C|SetActivationType _returnvalue "NewEnumerator3")
  (Default|CETrigger _returnvalue))

(event Collision|EventActorBeginOverlap
  (params (OtherActor :type Actor%20Object%20Reference)))

(event EventTick
  (params (DeltaSeconds :type Float%20%28single-precision%29)))

(fn ConstructionScript)