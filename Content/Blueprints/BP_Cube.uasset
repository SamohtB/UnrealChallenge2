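; BP_Cube is a breakable cube actor that drops a random power-up when its Chaos geometry collection fractures.
; The first break event on the geometry collection sets an IsBroken guard, calls GenerateItem and plays a collapse sound.
; GenerateItem picks one of four power-up cube Blueprints at random and spawns it with the scene root's relative transform, ignoring collisions.
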(event OnChaosBreakEvent(Cube32_GeometryCollection)
  (params (BreakEvent :type Chaos%20Break%20Event%20Structure%20%28by%20ref%29))
  (if (not (Variables|Default|GetisBroken))
    (Variables|Default|SetisBroken true)
    (CallFunction|GenerateItem)
    (Audio|PlaySoundatLocation "/Game/StarterContent/Audio/Collapse01.Collapse01" "0, 0, 0" "0, 0, 0" 0.5 1.0 0.0 0 0 0 0)))

(event Custom|Generate%20Item
  (bind _defaultsceneroot (Variables|Default|GetDefaultSceneRoot))
  (bind _returnvalue (Transformation|GetRelativeTransform _defaultsceneroot))
  (switch int (Math|Random|RandomInteger 4)
    (:0
      (Game|SpawnActorfromClass "/Game/FirstPerson/Blueprints/BP_PowerUp_Cube.BP_PowerUp_Cube_C" _returnvalue "AlwaysSpawn" 0 0))
    (:1
      (Game|SpawnActorfromClass "/Game/FirstPerson/Blueprints/BP_PowerUp_Cube_2.BP_PowerUp_Cube_2_C" _returnvalue "AlwaysSpawn" 0 0))
    (:2
      (Game|SpawnActorfromClass "/Game/FirstPerson/Blueprints/BP_PowerUp_Cube_3.BP_PowerUp_Cube_3_C" _returnvalue "AlwaysSpawn" 0 0))
    (:3
      (Game|SpawnActorfromClass "/Game/FirstPerson/Blueprints/BP_PowerUp_Cube_4.BP_PowerUp_Cube_4_C" _returnvalue "AlwaysSpawn" 0 0))))

(event EventBeginPlay)

(event Collision|EventActorBeginOverlap
  (params (OtherActor :type Actor%20Object%20Reference)))

(event EventTick
  (params (DeltaSeconds :type Float%20%28single-precision%29)))

(fn ConstructionScript)